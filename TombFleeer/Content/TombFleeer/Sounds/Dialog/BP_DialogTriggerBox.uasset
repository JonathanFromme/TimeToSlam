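; Trigger box that plays a one-shot dialog sound when the player character overlaps it.
; The hand-over dialog requires the cat statue, organ jar and treasure, and the farewell dialog requires the victory flag; other dialogs play unconditionally.
; After playback it disables itself and, depending on MummyShouldMove, teleports the first Mummy-tagged actor to a hardcoded location and rotation.
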(event EventBeginPlay)

(event Collision|EventActorBeginOverlap
  (params (OtherActor :type Actor%20Object%20Reference))
  (bind _returnvalue (Game|GetPlayerCharacter 0))
  (if (Variables|Default|GetShouldPlayDialogOnContact)
    (if (== OtherActor _returnvalue)
      (bind _asbp_first_person_character (Utilities|Casting|CastToBP_FirstPersonCharacter _returnvalue))
      (if (== (Variables|Default|GetDialogToPlay) "/Game/TombFleeer/Sounds/Dialog/Hand_To_Me_Dialog.Hand_To_Me_Dialog")
        (if (Math|Boolean|ANDBoolean (Variables|/Game/FirstPerson/Blueprints/BP_FirstPersonCharacter.BP_FirstPersonCharacter_C|GetHasCatStatue _asbp_first_person_character) (Variables|/Game/FirstPerson/Blueprints/BP_FirstPersonCharacter.BP_FirstPersonCharacter_C|GetHasOrganJar _asbp_first_person_character) (Variables|/Game/FirstPerson/Blueprints/BP_FirstPersonCharacter.BP_FirstPersonCharacter_C|GetHasTreasure _asbp_first_person_character))
          (Default|PlaySound _asbp_first_person_character (Variables|Default|GetDialogToPlay) :!label _label)
          (Variables|Default|SetShouldPlayDialogOnContact false)
          (bind _outactors (Actor|GetAllActorswithTag "Mummy"))
          (switch string (Variables|Default|GetMummyShouldMove)
            (:ControlPanel
              (Transformation|SetActorLocationAndRotation (Utilities|Array|Get(acopy) _outactors) "-1356.333140,2544.433083,12.066599" "0.000000,-129.999999,0.000000"))))
        (elif (== (Variables|Default|GetDialogToPlay) "/Game/TombFleeer/Sounds/Dialog/SeeYouNever_Dialog.SeeYouNever_Dialog")
          (if (Variables|/Game/TombFleeer/Responders/BP_VictoryText.BP_VictoryText_C|GetHasWon (Variables|Default|GetVictoryText))
            (goto _label))
          (else
            (goto _label)))))))

(event EventTick
  (params (DeltaSeconds :type Float%20%28single-precision%29)))

(fn ConstructionScript)