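; BP_VictoryText is a responder actor that runs the game's win sequence once the cat statue, organ jar and treasure pillars are all activated.
; Respond checks the three pillars, makes its root component visible and destroys every actor tagged DestroyOnWin.
; It then has the Mummy speak the last-item dialog, waits, plays the ending sound and adds the player character's Credits widget to the viewport.
; CanRespond always returns false.
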(event EventBeginPlay)

(event Collision|EventActorBeginOverlap
  (params (OtherActor :type Actor%20Object%20Reference)))

(event EventTick
  (params (DeltaSeconds :type Float%20%28single-precision%29)))

(event EventRespond
  (params (Controller%20Type :type E_ControllerTypes%20Enum :default "NewEnumerator0") (Value :type Float%20%28double-precision%29))
  (if (Math|Boolean|ANDBoolean (Variables|/Game/TombFleeer/Interactables/BP_MI_Pedestal.BP_MI_Pedestal_C|GetActivated (Variables|Default|GetCatStatuePillar)) (Variables|/Game/TombFleeer/Interactables/BP_MI_Pedestal.BP_MI_Pedestal_C|GetActivated (Variables|Default|GetOrganJarPillar)) (Variables|/Game/TombFleeer/Interactables/BP_MI_Pedestal.BP_MI_Pedestal_C|GetActivated (Variables|Default|GetTreasurePillar)))
    (Rendering|SetVisibility (Variables|Default|GetDefaultSceneRoot) true false)
    (bind _outactors (Actor|GetAllActorswithTag "DestroyOnWin"))
    (for _array_element _outactors
      (Actor|DestroyActor _array_element))
    (bind _asbp_first_person_character (Utilities|Casting|CastToBP_FirstPersonCharacter (Game|GetPlayerCharacter 0)))
    (Default|Speak (Variables|Default|GetMummy) "/Game/TombFleeer/Sounds/Dialog/Last_Item_Placed_Dialog.Last_Item_Placed_Dialog")
    (Utilities|FlowControl|Delay 15.0)
    (Audio|PlaySound2D "/Game/TombFleeer/Sounds/Music/Tomb_Service_Ending_Screen.Tomb_Service_Ending_Screen" 1.0 1.0 0.0 0 0)
    (UserInterface|Viewport|AddtoViewport (Variables|/Game/FirstPerson/Blueprints/BP_FirstPersonCharacter.BP_FirstPersonCharacter_C|GetCredits _asbp_first_person_character) 0)))

(fn ConstructionScript)

(fn CanRespond
  (return false))