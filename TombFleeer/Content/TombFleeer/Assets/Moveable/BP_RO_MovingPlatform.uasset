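; BP_RO_MovingPlatform is a responder actor that moves its Jug component as a platform in response to button or lever input.
; Button presses alternate between playing and stopping a timeline and an attached looping sound.
; The timeline drives the platform along world X toward DestinationCube while incrementally rotating three building-part meshes.
; Lever values are normalized to set world Y between the actor's location and LeverDestination, with debug prints left in.
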(event EventBeginPlay
  (|CallParentFunction) ; This node is disabled and will not be called.\nDrag off pins to build functionality.
)

(event Collision|EventActorBeginOverlap
  (params (OtherActor :type Actor%20Object%20Reference))
  (|CallParentFunction OtherActor) ; This node is disabled and will not be called.\nDrag off pins to build functionality.
)

(event EventTick
  (params (DeltaSeconds :type Float%20%28single-precision%29))
  (|CallParentFunction DeltaSeconds) ; This node is disabled and will not be called.\nDrag off pins to build functionality.
)

(event EventRespond
  (params (Controller%20Type :type E_ControllerTypes%20Enum :default "NewEnumerator0") (Value :type Float%20%28double-precision%29))
  (bind _returnvalue (Math|Float|NormalizetoRange Value 0.0 4.0))
  (bind _returnvalue_2 (Transformation|GetActorLocation))
  (bind _defaultsceneroot (Variables|Default|GetDefaultSceneRoot))
  (bind _leverdestination (Variables|Default|GetLeverDestination))
  (bind _jug (Variables|Default|GetJug))
  (bind _jug_2 (Variables|Default|GetJug))
  (bind _returnvalue_3 (Transformation|GetWorldTransform _defaultsceneroot))
  (bind _returnvalue_4 (Math|Vector|Lerp(Vector) _returnvalue_2 _leverdestination _returnvalue))
  (bind _returnvalue_5 (Transformation|GetWorldTransform _jug_2))
  (bind _returnvalue_6 (Transformation|GetWorldLocation _jug))
  (switch Utilities|FlowControl|Switch|SwitchonE_ControllerTypes Controller%20Type
    (:NewEnumerator0
      ;[0.15 0.15 0.15 0.5] Button Interactione
      (Utilities|FlowControl|FlipFlop
        (:A
          (bind _returnvalue_7 (Audio|SpawnSoundAttached "/Game/TombFleeer/Sounds/Foley/Push/MS_MovingPedestalLoop.MS_MovingPedestalLoop" (Variables|Default|GetJug) "Sphere" (Transformation|GetActorLocation) "0, 0, 0" "SnapToTarget" false 1.0 1.0 0.0 "/Game/TombFleeer/Sounds/Foley/Attenuation/SA_MovingObject.SA_MovingObject" 0))
          (bind _alpha (Timeline|Timeline Play)
            (:Update
              (Transformation|SetWorldTransform (Variables|Default|GetJug) (Math|Transform|MakeTransform (Math|Vector|MakeVector (Math|Float|Lerp (.X (Math|Vector|BreakVector (.location _returnvalue_3))) (.x (.location (Class|KismetMathLibrary|TInterpto (Math|Transform|MakeTransform (.location _returnvalue_3) "0, 0, 0" "1.000000,1.000000,1.000000") (Transformation|GetWorldTransform (Variables|Default|GetDestinationCube)) 0.0 0.0))) _alpha) (.y (.location _returnvalue_5)) (.z (.location _returnvalue_5))) (.rotation _returnvalue_5) (.scale _returnvalue_5)) false false)
              (for _array_element (Utilities|Array|MakeArray (Variables|Default|GetSM_building_part_010) (Variables|Default|GetSM_building_part_011) (Variables|Default|GetSM_building_part_09))
                (Transformation|SetWorldRotation _array_element (Math|Rotator|MakeRotator 9e+01 (+ (.pitch (Transformation|GetWorldRotation _array_element)) (Math|Float|MapRangeClamped _alpha 0.0 1.0 -1.0 1.0)) 0.0) false false)
                (Development|PrintString (Utilities|String|ToString(Float) (+ (.pitch (Transformation|GetWorldRotation _array_element)) (Math|Float|MapRangeClamped _alpha 0.0 1.0 -1.0 1.0))))))))
        (:B
          (Audio|Components|Audio|Stop _returnvalue_7)
          (Timeline|Timeline Stop))))
    (:NewEnumerator1
      ;[0.15 0.15 0.15 0.5] Lever Interaction - Move platform in Y direction
      (Transformation|SetWorldLocation _jug (Math|Vector|MakeVector (.x _returnvalue_6) (.y _returnvalue_4) (.z _returnvalue_6)) false false)
      (Development|PrintString (Utilities|String|ToString(Float) (.y _returnvalue_4))))))

(fn ConstructionScript
  (|CallParentFunction))

(fn CanRespond
  (return true))