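; BP_RO_Platform is a moveable platform that rotates a quarter turn each time its Respond event fires.
; Respond adds 90 degrees to the actor's pitch in one instant transform set, keeping location, roll and yaw, with no interpolation.
; It then plays the rotating-platform sound at the actor's location with moving-object attenuation.
; BeginPlay, overlap and Tick are disabled stubs, so Respond drives all behavior.
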(event EventBeginPlay
  (|CallParentFunction) ; This node is disabled and will not be called.\nDrag off pins to build functionality.
)

(event Collision|EventActorBeginOverlap
  (params (OtherActor :type Actor%20Object%20Reference))
  (|CallParentFunction OtherActor) ; This node is disabled and will not be called.\nDrag off pins to build functionality.
)

(event EventTick
  (params (DeltaSeconds :type Float%20%28single-precision%29))
  (|CallParentFunction DeltaSeconds) ; This node is disabled and will not be called.\nDrag off pins to build functionality.
)

(event EventRespond
  (params (Controller%20Type :type E_ControllerTypes%20Enum :default "NewEnumerator0") (Value :type Float%20%28double-precision%29))
  (bind _returnvalue (Transformation|GetActorTransform))
  ;[0.15 0.15 0.15 0.5] Rotate Object - leave it alone, it works
  (Transformation|SetActorTransform (Math|Transform|MakeTransform (.location _returnvalue) (Math|Rotator|MakeRotator (.roll (.rotation _returnvalue)) (+ (.pitch (.rotation _returnvalue)) 9e+01) (.yaw (.rotation _returnvalue))) "1.000000,1.000000,1.000000"))
  (Audio|SpawnSoundatLocation "/Game/TombFleeer/Sounds/Foley/Push/MS_rotatingPlatform.MS_rotatingPlatform" (Transformation|GetActorLocation) "0, 0, 0" 1.0 1.0 0.0 "/Game/TombFleeer/Sounds/Foley/Attenuation/SA_MovingObject.SA_MovingObject" 0))

(fn ConstructionScript
  (|CallParentFunction))