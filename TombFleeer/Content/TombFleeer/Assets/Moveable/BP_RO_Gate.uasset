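; BP_RO_Gate is a gate that toggles between its starting height and a lowered position each time it is told to respond.
; BeginPlay caches the root's world location, and a FlipFlop in Respond picks the target height, which is applied instantly with no interpolation.
; Respond also prints the new height and, if CanMakeNoise is set, plays an attenuated gate sound at the actor.
; CanRespond always returns true.
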(event EventBeginPlay
  (|CallParentFunction)
  (Variables|Default|SetlocationOrig (Transformation|GetWorldLocation (Variables|Default|GetDefaultSceneRoot))))

(event Collision|EventActorBeginOverlap
  (params (OtherActor :type Actor%20Object%20Reference))
  (|CallParentFunction OtherActor) ; This node is disabled and will not be called.\nDrag off pins to build functionality.
)

(event EventTick
  (params (DeltaSeconds :type Float%20%28single-precision%29))
  (|CallParentFunction DeltaSeconds) ; This node is disabled and will not be called.\nDrag off pins to build functionality.
)

(event EventRespond
  (params (Controller%20Type :type E_ControllerTypes%20Enum :default "NewEnumerator0") (Value :type Float%20%28double-precision%29))
  (bind _locationorig (Variables|Default|GetlocationOrig))
  (bind _isa (Utilities|FlowControl|FlipFlop)
    (:A
      _)
    (:B
      _))
  (Transformation|SetWorldLocation (Variables|Default|GetDefaultSceneRoot) (Math|Vector|MakeVector (.x _locationorig) (.y _locationorig) (select _isa (- (.z _locationorig) 1.7e+02) (.z _locationorig))) false false)
  (Development|PrintString (Utilities|String|ToString(Float) (select _isa (- (.z _locationorig) 1.7e+02) (.z _locationorig))))
  (if (Variables|Default|GetCanMakeNoise)
    (Audio|SpawnSoundatLocation "/Game/TombFleeer/Sounds/Foley/Push/MS_Gate.MS_Gate" (Transformation|GetActorLocation) "0, 0, 0" 1.0 1.0 1.0 "/Game/TombFleeer/Sounds/Foley/Attenuation/SA_MovingObject.SA_MovingObject" 0)))

(fn ConstructionScript
  (|CallParentFunction))

(fn CanRespond
  (return true))