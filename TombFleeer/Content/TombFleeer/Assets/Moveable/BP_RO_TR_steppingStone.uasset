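; Stepping stone Blueprint that slides its block mesh in and out along its local X axis each time Respond is called.
; A FlipFlop alternately plays and reverses a Timeline whose alpha scales the relative X offset of SMBlock03.
; The GoingOut flag records direction, but both of its branches apply the same movement.
; An attenuated platform sound is spawned attached to the block on every Timeline update, rather than once per move.
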(event EventBeginPlay
  (|CallParentFunction))

(event Collision|EventActorBeginOverlap
  (params (OtherActor :type Actor%20Object%20Reference))
  (|CallParentFunction OtherActor) ; This node is disabled and will not be called.\nDrag off pins to build functionality.
)

(event EventTick
  (params (DeltaSeconds :type Float%20%28single-precision%29))
  (|CallParentFunction DeltaSeconds) ; This node is disabled and will not be called.\nDrag off pins to build functionality.
)

(event EventRespond
  (params (Controller%20Type :type E_ControllerTypes%20Enum :default "NewEnumerator0") (Value :type Float%20%28double-precision%29))
  (bind _sm_block_03 (Variables|Default|GetSM_block_03))
  (Utilities|FlowControl|FlipFlop
    (:A
      (Variables|Default|SetgoingOut false)
      (bind _alpha (Timeline|Timeline Play)
        (:Update
          (if (Variables|Default|GetgoingOut)
            (Transformation|SetRelativeLocation _sm_block_03 (Math|Vector|MakeVector (* _alpha -7e+01) 0.0 0.0) false false)
            (else
              (Transformation|SetRelativeLocation _sm_block_03 (Math|Vector|MakeVector (* _alpha -7e+01) 0.0 0.0) false false)))
          (Audio|SpawnSoundAttached "/Game/TombFleeer/Sounds/Foley/Push/MS_Platforms.MS_Platforms" (Variables|Default|GetSM_block_03) "None" "0, 0, 0" "0, 0, 0" "KeepRelativeOffset" false 1.0 1.0 0.0 "/Game/TombFleeer/Sounds/Foley/Attenuation/SA_Platforms.SA_Platforms" 0))))
    (:B
      (Variables|Default|SetgoingOut true)
      (Timeline|Timeline Reverse))))

(fn ConstructionScript
  (|CallParentFunction))