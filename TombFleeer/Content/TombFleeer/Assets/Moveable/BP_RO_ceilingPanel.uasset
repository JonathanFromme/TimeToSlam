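; BP_RO_ceilingPanel is a responder actor for a ceiling panel that rotates according to an incoming value.
; Respond remaps the value from a -180 to 180 range onto 0 to 360 degrees and sets it as the static mesh's world yaw, with roll fixed at 90.
; It also prints the computed angle, and CanRespond always returns true.
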(event EventBeginPlay
  (|CallParentFunction) ; This node is disabled and will not be called.\nDrag off pins to build functionality.
)

(event Collision|EventActorBeginOverlap
  (params (OtherActor :type Actor%20Object%20Reference))
  (|CallParentFunction OtherActor) ; This node is disabled and will not be called.\nDrag off pins to build functionality.
)

(event EventTick
  (params (DeltaSeconds :type Float%20%28single-precision%29))
  (|CallParentFunction DeltaSeconds) ; This node is disabled and will not be called.\nDrag off pins to build functionality.
)

(event EventRespond
  (params (Controller%20Type :type E_ControllerTypes%20Enum :default "NewEnumerator0") (Value :type Float%20%28double-precision%29))
  (bind _returnvalue (Math|Float|NormalizetoRange Value -1.8e+02 1.8e+02))
  (bind _returnvalue_2 (* _returnvalue 3.6e+02))
  (bind _returnvalue_3 (+ _returnvalue_2 0.0))
  (Transformation|SetWorldRotation (Variables|Default|GetStaticMesh) (Math|Rotator|MakeRotator 9e+01 0.0 _returnvalue_3) false false)
  (Development|PrintString (Utilities|String|ToString(Float) _returnvalue_3)))

(fn ConstructionScript
  (|CallParentFunction))

(fn CanRespond
  (return true))