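; BP_RO_RotatingPlatform is a moveable platform that rotates in response to an incoming value.
; Its Respond event sets the world rotation of the SMBuildingPart05 component, using the value as an absolute pitch and zeroing roll and yaw.
; The event also prints the value to screen, while BeginPlay, overlap and Tick are disabled stubs.
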(event EventBeginPlay
  (|CallParentFunction) ; This node is disabled and will not be called.\nDrag off pins to build functionality.
)

(event Collision|EventActorBeginOverlap
  (params (OtherActor :type Actor%20Object%20Reference))
  (|CallParentFunction OtherActor) ; This node is disabled and will not be called.\nDrag off pins to build functionality.
)

(event EventTick
  (params (DeltaSeconds :type Float%20%28single-precision%29))
  (|CallParentFunction DeltaSeconds) ; This node is disabled and will not be called.\nDrag off pins to build functionality.
)

(event EventRespond
  (params (Controller%20Type :type E_ControllerTypes%20Enum :default "NewEnumerator0") (Value :type Float%20%28double-precision%29))
  (Transformation|SetWorldRotation (Variables|Default|GetSM_building_part_05) (Math|Rotator|MakeRotator 0.0 Value 0.0) false false)
  (Development|PrintString (Utilities|String|ToString(Float) Value)))

(fn ConstructionScript
  (|CallParentFunction))