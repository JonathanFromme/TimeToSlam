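; BP_RO_light is a responder light in TombFleeer that switches a visible light cone and feeds a connected pedestal.
; Respond treats the incoming value as an angle in degrees, counting it as lit when its sine falls inside symmetric positive or negative bands.
; That result sets the cone material's opacity fully on or off, flags the pedestal as receiving light and calls its UpdateLight.
; CanRespond always returns true.
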(event EventBeginPlay
  (|CallParentFunction) ; This node is disabled and will not be called.\nDrag off pins to build functionality.
)

(event Collision|EventActorBeginOverlap
  (params (OtherActor :type Actor%20Object%20Reference))
  (|CallParentFunction OtherActor) ; This node is disabled and will not be called.\nDrag off pins to build functionality.
)

(event EventTick
  (params (DeltaSeconds :type Float%20%28single-precision%29))
  (|CallParentFunction DeltaSeconds) ; This node is disabled and will not be called.\nDrag off pins to build functionality.
)

(event EventRespond
  (params (Controller%20Type :type E_ControllerTypes%20Enum :default "NewEnumerator0") (Value :type Float%20%28double-precision%29))
  (bind _returnvalue (Math|Trig|Sin(Degrees) Value))
  (bind _connectedpedestal (Variables|Default|GetConnectedPedestal))
  (bind _returnvalue_2 (> _returnvalue -0.98))
  (bind _returnvalue_3 (< _returnvalue -0.15))
  (bind _returnvalue_4 (> _returnvalue 0.15))
  (bind _returnvalue_5 (< _returnvalue 0.98))
  (bind _returnvalue_6 (and _returnvalue_2 _returnvalue_3))
  (bind _returnvalue_7 (and _returnvalue_4 _returnvalue_5))
  (bind _returnvalue_8 (or _returnvalue_7 _returnvalue_6))
  (bind _returnvalue_9 (Math|Float|SelectFloat 1.0 0.0 _returnvalue_8))
  (Rendering|Material|SetScalarParameterValueonMaterials (Variables|Default|GetCone) "Opacity" _returnvalue_9)
  (Variables|/Game/TombFleeer/Assets/Moveable/BP_RO_Pedestal.BP_RO_Pedestal_C|SetIsReceivingLight _connectedpedestal _returnvalue_8)
  (Default|UpdateLight _connectedpedestal _returnvalue_9))

(fn ConstructionScript
  (|CallParentFunction))

(fn CanRespond
  (return true))