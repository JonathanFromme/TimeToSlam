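; BP_RO_Text is a responding object that shows or hides a text render component according to the value it receives.
; Respond makes the text visible only when the value minus one equals three, and hides it for any other value.
; CanRespond always returns true, and the stock BeginPlay, overlap and Tick events are disabled.
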(event EventBeginPlay
  (|CallParentFunction) ; This node is disabled and will not be called.\nDrag off pins to build functionality.
)

(event Collision|EventActorBeginOverlap
  (params (OtherActor :type Actor%20Object%20Reference))
  (|CallParentFunction OtherActor) ; This node is disabled and will not be called.\nDrag off pins to build functionality.
)

(event EventTick
  (params (DeltaSeconds :type Float%20%28single-precision%29))
  (|CallParentFunction DeltaSeconds) ; This node is disabled and will not be called.\nDrag off pins to build functionality.
)

(event EventRespond
  (params (Controller%20Type :type E_ControllerTypes%20Enum :default "NewEnumerator0") (Value :type Float%20%28double-precision%29))
  (Rendering|SetVisibility (Variables|Default|GetTextRender) (== (- Value 1.0) 3.0) false))

(fn ConstructionScript
  (|CallParentFunction))

(fn CanRespond
  (return true))