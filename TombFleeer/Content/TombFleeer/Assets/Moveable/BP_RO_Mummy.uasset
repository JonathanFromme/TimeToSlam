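; BP_RO_Mummy is a talking mummy actor that turns to face the player and plays voice lines on request.
; Tick smoothly interpolates only its yaw toward the player character.
; Speak stops any line still playing, stores the new attached, attenuated sound, and plays it.
; The first interruption also plays a one-time Scarab_Dialog complaint, delaying the new line until it has had time to play.
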(event Custom|Speak
  (params (SoundToPlay :type Sound%20Wave%20Object%20Reference))
  (Utilities|IsValid (Variables|Default|GetPreviousAudio)
    (:Is%20Valid
      (if (Audio|Components|Audio|IsPlaying (Variables|Default|GetPreviousAudio))
        (Audio|Components|Audio|Stop (Variables|Default|GetPreviousAudio))
        (if (Variables|Default|GetHasPlayedComplaint)
          _
          (else
            (Variables|Default|SetHasPlayedComplaint true)
            (Audio|SpawnSoundAttached "/Game/TombFleeer/Sounds/Dialog/Scarab_Dialog.Scarab_Dialog" (Variables|Default|GetAudio) "None" (Transformation|GetActorLocation) "0, 0, 0" "KeepRelativeOffset" false 1.0 1.0 0.0 "/Game/TombFleeer/Sounds/Dialog/SA_Mummy.SA_Mummy" 0)
            (Utilities|FlowControl|Delay 5.0)))))
    (:Is%20Not%20Valid
      _))
  (bind _returnvalue (Audio|SpawnSoundAttached SoundToPlay (Variables|Default|GetAudio) "None" (Transformation|GetActorLocation) "0, 0, 0" "KeepRelativeOffset" false 1.0 1.0 0.0 "/Game/TombFleeer/Sounds/Dialog/SA_Mummy.SA_Mummy" 0))
  (Variables|Default|SetPreviousAudio _returnvalue))

(event EventBeginPlay
  (|CallParentFunction))

(event Collision|EventActorBeginOverlap
  (params (OtherActor :type Actor%20Object%20Reference))
  (|CallParentFunction OtherActor) ; This node is disabled and will not be called.\nDrag off pins to build functionality.
)

(event EventTick
  (params (DeltaSeconds :type Float%20%28single-precision%29))
  (|CallParentFunction DeltaSeconds)
  (Transformation|SetActorRotation (Math|Rotator|MakeRotator 0.0 0.0 (.yaw (Math|Interpolation|RInterpTo (Transformation|GetActorRotation) (Math|Rotator|FindLookatRotation (Transformation|GetActorLocation) (Transformation|GetActorLocation (Game|GetPlayerCharacter 0))) (Utilities|Time|GetWorldDeltaSeconds) 5.0)))))

(fn ConstructionScript
  (|CallParentFunction))