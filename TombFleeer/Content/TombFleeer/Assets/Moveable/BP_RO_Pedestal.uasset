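; BP_RO_Pedestal is a responder puzzle pedestal that reacts to lever, dial and button messages.
; Levers slide it along Y from its start, dials yaw its block, and buttons refresh the light cone, shown only when lit at position 3.
; After a delay, UpdateGem also requires yaw near 180 degrees to make GlowJewel's material a gem.
; The first success plays a chime and messages RotatingRectangle.
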(event EventBeginPlay
  (|CallParentFunction)
  (Variables|Default|SetlocationOrig (Transformation|GetWorldLocation (Variables|Default|GetDefaultSceneRoot)))
  (Rendering|SetVisibility (Variables|Default|GetCone) false false))

(event Collision|EventActorBeginOverlap
  (params (OtherActor :type Actor%20Object%20Reference))
  (|CallParentFunction OtherActor) ; This node is disabled and will not be called.\nDrag off pins to build functionality.
)

(event EventTick
  (params (DeltaSeconds :type Float%20%28single-precision%29))
  (|CallParentFunction DeltaSeconds) ; This node is disabled and will not be called.\nDrag off pins to build functionality.
)

(event EventRespond
  (params (Controller%20Type :type E_ControllerTypes%20Enum :default "NewEnumerator0") (Value :type Float%20%28double-precision%29))
  (bind _locationorig (Variables|Default|GetlocationOrig))
  (switch Utilities|FlowControl|Switch|SwitchonE_ControllerTypes Controller%20Type
    (:NewEnumerator0
      (if (Variables|Default|GetIsReceivingLight) :!label _label
        (Rendering|SetVisibility (Variables|Default|GetCone) (== (Variables|Default|GetPosition) 3.0) false)
        (Rendering|Material|SetScalarParameterValueonMaterials (Variables|Default|GetCone) "Opacity" (Math|Conversions|ToFloat(Boolean) (== (Variables|Default|GetPosition) 3.0)))
        (Utilities|FlowControl|Delay 2.0)
        (CallFunction|UpdateGem)
        (else
          (Utilities|FlowControl|Delay 2.0)
          (CallFunction|UpdateGem))))
    (:NewEnumerator1
      (Variables|Default|SetPosition Value)
      (Utilities|FlowControl|Sequence
        (:then_0
          (goto _label))
        (:then_1
          (Transformation|SetWorldLocation (Variables|Default|GetDefaultSceneRoot) (Math|Vector|MakeVector (.x _locationorig) (+ (.y _locationorig) (* Value (Variables|Default|GetDistance))) (.z _locationorig)) false false)
          (Audio|SpawnSoundatLocation "/Game/TombFleeer/Sounds/Foley/Push/MS_MovingPedestal.MS_MovingPedestal" (Transformation|GetActorLocation) "0, 0, 0" (Variables|Default|GetVolume%20Multiplier) 1.0 1.0 "/Game/TombFleeer/Sounds/Foley/Attenuation/SA_MovingObject.SA_MovingObject" 0)
          (Utilities|FlowControl|Delay 2.0)
          (CallFunction|UpdateGem))))
    (:NewEnumerator2
      (Transformation|SetWorldRotation (Variables|Default|GetSM_block_09) (Math|Rotator|MakeRotator 0.0 0.0 Value) false false)
      (Utilities|FlowControl|Delay 2.0)
      (CallFunction|UpdateGem))))

(fn ConstructionScript
  (|CallParentFunction))

(fn CanRespond
  (return true))

(fn UpdateLight
  (params (Float :type Float%20%28double-precision%29))
  (if (Variables|Default|GetIsReceivingLight)
    (if (== (Variables|Default|GetPosition) 3.0)
      (Rendering|SetVisibility (Variables|Default|GetCone) true false)
      (Rendering|Material|SetScalarParameterValueonMaterials (Variables|Default|GetCone) "Opacity" Float)
      (else
        (Rendering|SetVisibility (Variables|Default|GetCone) false false :!label _label)))
    (else
      (goto _label))))

(fn UpdateGem
  (bind _glowjewel (Variables|Default|GetGlowJewel))
  (bind _sm_block_09 (Variables|Default|GetSM_block_09))
  (bind _glowjewel_2 (Variables|Default|GetGlowJewel))
  (bind _returnvalue (Transformation|GetWorldRotation _sm_block_09))
  (if (Math|Boolean|ANDBoolean (Variables|Default|GetIsReceivingLight) (or (and (>= (.yaw _returnvalue) 175.0) (<= (.yaw _returnvalue) 1.8e+02)) (and (>= (.yaw _returnvalue) -1.8e+02) (<= (.yaw _returnvalue) -175.0))) (== (Variables|Default|GetPosition) 3.0))
    (Rendering|Material|SetMaterial (Variables|/Script/Engine.StaticMeshActor|GetStaticMeshComponent _glowjewel) 0 "/Game/TombFleeer/Materials/Instances/MI_Gem.MI_Gem")
    (Rendering|Material|SetMaterial (Variables|/Script/Engine.StaticMeshActor|GetStaticMeshComponent _glowjewel) 2 "/Game/TombFleeer/Materials/Instances/MI_Gem.MI_Gem")
    (Rendering|Material|SetMaterial (Variables|/Script/Engine.StaticMeshActor|GetStaticMeshComponent _glowjewel) 3 "/Game/TombFleeer/Materials/Instances/MI_Gem.MI_Gem")
    (Rendering|Material|SetMaterial (Variables|/Script/Engine.StaticMeshActor|GetStaticMeshComponent _glowjewel) 4 "/Game/TombFleeer/Materials/Instances/MI_Gem.MI_Gem")
    (if (not (Variables|Default|GetDoOnce))
      (Class|BPIResponder|Respond(Message) (Variables|Default|GetRotatingRectangle) "NewEnumerator0" 0.0)
      (Audio|PlaySoundatLocation "/Game/TombFleeer/Sounds/Foley/gjfx_success_chime.gjfx_success_chime" (Transformation|GetActorLocation) "0, 0, 0" 1.0 1.0 0.0 "/Game/TombFleeer/Sounds/Dialog/SA_Mummy.SA_Mummy" 0 0 0)
      (Variables|Default|SetDoOnce true))
    (else
      (Rendering|Material|SetMaterial (Variables|/Script/Engine.StaticMeshActor|GetStaticMeshComponent _glowjewel_2) 0 "/Game/Stylized_Egypt/Materials/building_materials/base_materials/MI_metal_A_Inst.MI_metal_A_Inst")
      (Rendering|Material|SetMaterial (Variables|/Script/Engine.StaticMeshActor|GetStaticMeshComponent _glowjewel_2) 2 "/Game/Stylized_Egypt/Materials/building_materials/base_materials/MI_metal_A_Inst.MI_metal_A_Inst")
      (Rendering|Material|SetMaterial (Variables|/Script/Engine.StaticMeshActor|GetStaticMeshComponent _glowjewel_2) 3 "/Game/Stylized_Egypt/Materials/building_materials/base_materials/MI_metal_A_Inst.MI_metal_A_Inst")
      (Rendering|Material|SetMaterial (Variables|/Script/Engine.StaticMeshActor|GetStaticMeshComponent _glowjewel_2) 4 "/Game/Stylized_Egypt/Materials/building_materials/base_materials/MI_metal_A_Inst.MI_metal_A_Inst"))))