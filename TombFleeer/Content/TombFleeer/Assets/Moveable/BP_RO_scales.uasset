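; Interactable scales puzzle object that tips a little further each time a rock is added, up to five.
; Each Interact raises the rock count and sets a new target pitch, which Tick eases the mesh toward with RInterpTo.
; The fifth rock plays a success chime and, after a short delay, has the Mummy speak the judgement dialog.
; CanInteract simply returns the ReadyToInteract flag.
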(event EventBeginPlay
  (|CallParentFunction))

(event Collision|EventActorBeginOverlap
  (params (OtherActor :type Actor%20Object%20Reference))
  (|CallParentFunction OtherActor) ; This node is disabled and will not be called.\nDrag off pins to build functionality.
)

(event EventTick
  (params (DeltaSeconds :type Float%20%28single-precision%29))
  (bind _sm_building_border_05 (Variables|Default|GetSM_building_border_05))
  (|CallParentFunction DeltaSeconds)
  (Transformation|SetWorldRotation _sm_building_border_05 (Math|Interpolation|RInterpTo (Transformation|GetWorldRotation _sm_building_border_05) (Variables|Default|GetRotation) (Utilities|Time|GetWorldDeltaSeconds) 5.0) false false))

(event EventInteract
  (params (Amount :type Float%20%28double-precision%29))
  (bind _sm_building_border_05 (Variables|Default|GetSM_building_border_05))
  (bind _returnvalue (Transformation|GetWorldRotation _sm_building_border_05))
  (if (<= (Variables|Default|GetTotalRocks) 4)
    (Variables|Default|SetTotalRocks (+ (Variables|Default|GetTotalRocks) 1))
    (Variables|Default|SetRotation (Math|Rotator|MakeRotator (.roll _returnvalue) (+ (.pitch _returnvalue) 8.0) (.yaw _returnvalue)))
    (if (== (Variables|Default|GetTotalRocks) 5)
      (Audio|PlaySoundatLocation "/Game/TombFleeer/Sounds/Foley/gjfx_success_chime.gjfx_success_chime" (Transformation|GetActorLocation) "0, 0, 0" 1.0 1.0 0.0 0 0 0 0)
      (Utilities|FlowControl|Delay 2.5)
      (Default|Speak (Variables|Default|GetMummy) "/Game/TombFleeer/Sounds/Dialog/Scales_Judge_Dialog.Scales_Judge_Dialog"))))

(fn ConstructionScript
  (|CallParentFunction))

(fn CanInteract
  (return (Variables|Default|GetReadyToInteract)))