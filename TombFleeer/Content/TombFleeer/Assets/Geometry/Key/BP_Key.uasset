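; BP_Key is a key pickup actor that floats in place and turns to face the player.
; On BeginPlay it stores the key component's world position and plays a timeline whose Floating track, scaled by IncrementMovement, offsets the height.
; Each Tick it smoothly interpolates the actor's yaw toward player 0 with RInterpTo.
; It has no collection or overlap logic of its own.
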(event EventBeginPlay
  (Variables|Default|SetoriginalPos (Transformation|GetWorldLocation (Variables|Default|GetKey)))
  (bind _floating (Timeline|Timeline Play)
    (:Update
      (Transformation|SetWorldLocation (Variables|Default|GetKey) (Math|Vector|MakeVector (.X (Math|Vector|BreakVector (Variables|Default|GetoriginalPos))) (.Y (Math|Vector|BreakVector (Variables|Default|GetoriginalPos))) (+ (.Z (Math|Vector|BreakVector (Variables|Default|GetoriginalPos))) (* _floating (Variables|Default|GetIncrement%20Movement)))) false false))))

(event Collision|EventActorBeginOverlap
  (params (OtherActor :type Actor%20Object%20Reference)))

(event EventTick
  (params (DeltaSeconds :type Float%20%28single-precision%29))
  (Transformation|SetActorRotation (Math|Rotator|MakeRotator 0.0 0.0 (.yaw (Math|Interpolation|RInterpTo (Transformation|GetActorRotation) (Math|Rotator|FindLookatRotation (Transformation|GetActorLocation) (Transformation|GetActorLocation (Game|GetPlayerCharacter 0))) (Utilities|Time|GetWorldDeltaSeconds) 5.0)))))

(fn ConstructionScript)