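; Collectable interactable that is picked up when it receives the Interact event.
; Interact plays the configurable pickup sound at the location of its child actor, then destroys the collectable.
; It adds no inventory or score logic here, and its BeginPlay, overlap, Tick and construction script add no behavior of their own.
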(event EventBeginPlay
  (|CallParentFunction) ; This node is disabled and will not be called.\nDrag off pins to build functionality.
)

(event Collision|EventActorBeginOverlap
  (params (OtherActor :type Actor%20Object%20Reference))
  (|CallParentFunction OtherActor) ; This node is disabled and will not be called.\nDrag off pins to build functionality.
)

(event EventTick
  (params (DeltaSeconds :type Float%20%28single-precision%29))
  (|CallParentFunction DeltaSeconds) ; This node is disabled and will not be called.\nDrag off pins to build functionality.
)

(event EventInteract
  (params (Amount :type Float%20%28double-precision%29))
  (Audio|PlaySoundatLocation (Variables|Default|GetSoundToPlayOnPickup) (Transformation|GetActorLocation (Variables|/Script/Engine.ChildActorComponent|GetChildActor (Variables|Default|GetChildActor))) "0, 0, 0" 1.0 1.0 0.0 0 0 0 0)
  (Actor|DestroyActor))

(fn ConstructionScript
  (|CallParentFunction))