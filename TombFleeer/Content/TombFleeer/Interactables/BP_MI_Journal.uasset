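; Interactable journal actor that lets the player read a journal held in its child actor component.
; On Interact, it hides the quest marker on the BP_Journal child actor, then casts the player pawn to BP_FirstPersonCharacter.
; If the character is not already reading, it calls ReadJournal and plays an attenuated page-turn sound at the actor's location.
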(event EventBeginPlay)

(event Collision|EventActorBeginOverlap
  (params (OtherActor :type Actor%20Object%20Reference))
  (|CallParentFunction OtherActor) ; This node is disabled and will not be called.\nDrag off pins to build functionality.
)

(event EventTick
  (params (DeltaSeconds :type Float%20%28single-precision%29))
  (|CallParentFunction DeltaSeconds) ; This node is disabled and will not be called.\nDrag off pins to build functionality.
)

(event EventInteract
  (params (Amount :type Float%20%28double-precision%29))
  (bind _asbp_journal (Utilities|Casting|CastToBP_Journal (Variables|/Script/Engine.ChildActorComponent|GetChildActor (Variables|Default|GetChildActor))))
  (Rendering|SetVisibility (Variables|/Game/TombFleeer/Assets/Geometry/Journal/BP_Journal.BP_Journal_C|GetQuestMarker _asbp_journal) false false)
  (bind _asbp_first_person_character (Utilities|Casting|CastToBP_FirstPersonCharacter (Game|GetPlayerCharacter 0)))
  (if (not (Variables|/Game/FirstPerson/Blueprints/BP_FirstPersonCharacter.BP_FirstPersonCharacter_C|GetIsReadingJournal _asbp_first_person_character))
    (Default|ReadJournal _asbp_first_person_character)
    (Audio|SpawnSoundatLocation "/Game/TombFleeer/Sounds/Foley/PageTurn/MS_pageTurn.MS_pageTurn" (Transformation|GetActorLocation) "0, 0, 0" 1.0 1.0 0.0 "/Game/TombFleeer/Sounds/Foley/PageTurn/SA_pageTurn.SA_pageTurn" 0)))

(fn ConstructionScript
  (|CallParentFunction))