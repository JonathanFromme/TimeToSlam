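; Interactable multi-position lever that steps through three, four or five positions and reports its setting to connected actors.
; Interact is gated by ReadyToInteract, then branches on Positions and Current to play a timeline that rotates the child actor's "pullBar"-tagged meshes along roll.
; When each timeline finishes, Current advances, or wraps to 1 after the last position, and is sent to ConnectedActors through RespondMessage.
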(event EventBeginPlay
  (|CallParentFunction) ; This node is disabled and will not be called.\nDrag off pins to build functionality.
)

(event Collision|EventActorBeginOverlap
  (params (OtherActor :type Actor%20Object%20Reference))
  (|CallParentFunction OtherActor) ; This node is disabled and will not be called.\nDrag off pins to build functionality.
)

(event EventTick
  (params (DeltaSeconds :type Float%20%28single-precision%29))
  (|CallParentFunction DeltaSeconds) ; This node is disabled and will not be called.\nDrag off pins to build functionality.
)

(event EventInteract
  (params (Amount :type Float%20%28double-precision%29))
  (bind _childactor (Variables|Default|GetChildActor))
  (bind _childactor_2 (Variables|Default|GetChildActor))
  (bind _childactor_3 (Variables|Default|GetChildActor))
  (bind _childactor_4 (Variables|Default|GetChildActor))
  (bind _childactor_5 (Variables|Default|GetChildActor))
  (bind _childactor_6 (Variables|Default|GetChildActor))
  (bind _childactor_7 (Variables|Default|GetChildActor))
  (bind _childactor_8 (Variables|Default|GetChildActor))
  (bind _childactor_9 (Variables|Default|GetChildActor))
  (bind _childactor_10 (Variables|/Script/Engine.ChildActorComponent|GetChildActor _childactor))
  (bind _childactor_11 (Variables|/Script/Engine.ChildActorComponent|GetChildActor _childactor_2))
  (bind _childactor_12 (Variables|/Script/Engine.ChildActorComponent|GetChildActor _childactor_3))
  (bind _childactor_13 (Variables|/Script/Engine.ChildActorComponent|GetChildActor _childactor_4))
  (bind _childactor_14 (Variables|/Script/Engine.ChildActorComponent|GetChildActor _childactor_5))
  (bind _childactor_15 (Variables|/Script/Engine.ChildActorComponent|GetChildActor _childactor_6))
  (bind _childactor_16 (Variables|/Script/Engine.ChildActorComponent|GetChildActor _childactor_7))
  (bind _childactor_17 (Variables|/Script/Engine.ChildActorComponent|GetChildActor _childactor_8))
  (bind _childactor_18 (Variables|/Script/Engine.ChildActorComponent|GetChildActor _childactor_9))
  (bind _returnvalue (Actor|GetComponentsbyTag _childactor_11 "/Script/Engine.StaticMeshComponent" "pullBar"))
  (bind _returnvalue_2 (Actor|GetComponentsbyTag _childactor_12 "/Script/Engine.StaticMeshComponent" "pullBar"))
  (bind _returnvalue_3 (Actor|GetComponentsbyTag _childactor_13 "/Script/Engine.StaticMeshComponent" "pullBar"))
  (bind _returnvalue_4 (Actor|GetComponentsbyTag _childactor_14 "/Script/Engine.StaticMeshComponent" "pullBar"))
  (bind _returnvalue_5 (Actor|GetComponentsbyTag _childactor_15 "/Script/Engine.StaticMeshComponent" "pullBar"))
  (bind _returnvalue_6 (Actor|GetComponentsbyTag _childactor_16 "/Script/Engine.StaticMeshComponent" "pullBar"))
  (bind _returnvalue_7 (Actor|GetComponentsbyTag _childactor_17 "/Script/Engine.StaticMeshComponent" "pullBar"))
  (bind _returnvalue_8 (Actor|GetComponentsbyTag _childactor_10 "/Script/Engine.StaticMeshComponent" "pullBar"))
  (bind _returnvalue_9 (Actor|GetComponentsbyTag _childactor_18 "/Script/Engine.StaticMeshComponent" "pullBar"))
  (bind _output (Utilities|Array|Get(acopy) _returnvalue_8))
  (bind _output_2 (Utilities|Array|Get(acopy) _returnvalue))
  (bind _output_3 (Utilities|Array|Get(acopy) _returnvalue_2))
  (bind _output_4 (Utilities|Array|Get(acopy) _returnvalue_3))
  (bind _output_5 (Utilities|Array|Get(acopy) _returnvalue_4))
  (bind _output_6 (Utilities|Array|Get(acopy) _returnvalue_5))
  (bind _output_7 (Utilities|Array|Get(acopy) _returnvalue_6))
  (bind _output_8 (Utilities|Array|Get(acopy) _returnvalue_7))
  (bind _output_9 (Utilities|Array|Get(acopy) _returnvalue_9))
  (bind _relativerotation (Variables|/Script/Engine.SceneComponent|GetRelativeRotation _output))
  (bind _relativerotation_2 (Variables|/Script/Engine.SceneComponent|GetRelativeRotation _output_2))
  (bind _relativerotation_3 (Variables|/Script/Engine.SceneComponent|GetRelativeRotation _output_3))
  (bind _relativerotation_4 (Variables|/Script/Engine.SceneComponent|GetRelativeRotation _output_4))
  (bind _relativerotation_5 (Variables|/Script/Engine.SceneComponent|GetRelativeRotation _output_5))
  (bind _relativerotation_6 (Variables|/Script/Engine.SceneComponent|GetRelativeRotation _output_6))
  (bind _relativerotation_7 (Variables|/Script/Engine.SceneComponent|GetRelativeRotation _output_7))
  (bind _relativerotation_8 (Variables|/Script/Engine.SceneComponent|GetRelativeRotation _output_8))
  (bind _relativerotation_9 (Variables|/Script/Engine.SceneComponent|GetRelativeRotation _output_9))
  (if (Variables|Default|GetReadyToInteract)
    (Variables|Default|SetReadyToInteract false)
    (if (== (Variables|Default|GetPositions) 3)
      (switch int (Variables|Default|GetCurrent)
        (:1
          ;[0.15 0.15 0.15 0.5] 3 Section
          (bind _alpha (Timeline|Timeline_0 PlayFromStart)
            (:Update
              (Transformation|SetRelativeRotation (Actor|GetComponentsbyTag (Variables|/Script/Engine.ChildActorComponent|GetChildActor (Variables|Default|GetChildActor)) "/Script/Engine.StaticMeshComponent" "pullBar") (Math|Rotator|Lerp(Rotator) (Math|Rotator|MakeRotator (.roll _relativerotation_3) (.pitch _relativerotation_3) (.yaw _relativerotation_3)) (Math|Rotator|MakeRotator 0.0 (.pitch _relativerotation_3) (.yaw _relativerotation_3)) _alpha true) false false))
            (:Finished
              (Variables|Default|SetReadyToInteract true :!label _label)
              (Variables|Default|SetCurrent (+ (Variables|Default|GetCurrent) 1))
              (Class|BPIResponder|Respond(Message) (Variables|Default|GetConnectedActors) "NewEnumerator1" (Math|Conversions|ToFloat(Integer) (Variables|Default|GetCurrent))))))
        (:2
          (bind _alpha_2 (Timeline|Timeline_2 PlayFromStart)
            (:Update
              (Transformation|SetRelativeRotation (Actor|GetComponentsbyTag (Variables|/Script/Engine.ChildActorComponent|GetChildActor (Variables|Default|GetChildActor)) "/Script/Engine.StaticMeshComponent" "pullBar") (Math|Rotator|Lerp(Rotator) (Math|Rotator|MakeRotator (.roll _relativerotation_4) (.pitch _relativerotation_4) (.yaw _relativerotation_4)) (Math|Rotator|MakeRotator 4e+01 (.pitch _relativerotation_4) (.yaw _relativerotation_4)) _alpha_2 true) false false))
            (:Finished
              (goto _label))))
        (:3
          (bind _alpha_3 (Timeline|Timeline_1 PlayFromStart)
            (:Update
              (Transformation|SetRelativeRotation (Actor|GetComponentsbyTag (Variables|/Script/Engine.ChildActorComponent|GetChildActor (Variables|Default|GetChildActor)) "/Script/Engine.StaticMeshComponent" "pullBar") (Math|Rotator|Lerp(Rotator) "0.000000,0.000000,40.000000" "0.000000,0.000000,-40.000000" _alpha_3) false false))
            (:Finished
              (Variables|Default|SetReadyToInteract true)
              (Variables|Default|SetCurrent 1)
              (Class|BPIResponder|Respond(Message) (Variables|Default|GetConnectedActors) "NewEnumerator1" (Math|Conversions|ToFloat(Integer) (Variables|Default|GetCurrent)))))))
      (elif (== (Variables|Default|GetPositions) 4)
        (switch int (Variables|Default|GetCurrent)
          (:1
            ;[0.15 0.15 0.15 0.5] 4 Section
            (bind _alpha_4 (Timeline|Timeline_3 PlayFromStart)
              (:Update
                (Transformation|SetRelativeRotation (Actor|GetComponentsbyTag (Variables|/Script/Engine.ChildActorComponent|GetChildActor (Variables|Default|GetChildActor)) "/Script/Engine.StaticMeshComponent" "pullBar") (Math|Rotator|Lerp(Rotator) (Math|Rotator|MakeRotator (.roll _relativerotation_6) (.pitch _relativerotation_6) (.yaw _relativerotation_6)) (Math|Rotator|MakeRotator -13.333333 (.pitch _relativerotation_6) (.yaw _relativerotation_6)) _alpha_4 true) false false))
              (:Finished
                (Variables|Default|SetReadyToInteract true :!label _label_2)
                (Variables|Default|SetCurrent (+ (Variables|Default|GetCurrent) 1))
                (Class|BPIResponder|Respond(Message) (Variables|Default|GetConnectedActors) "NewEnumerator1" (Math|Conversions|ToFloat(Integer) (Variables|Default|GetCurrent))))))
          (:2
            (bind _alpha_5 (Timeline|Timeline_4 PlayFromStart)
              (:Update
                (Transformation|SetRelativeRotation (Actor|GetComponentsbyTag (Variables|/Script/Engine.ChildActorComponent|GetChildActor (Variables|Default|GetChildActor)) "/Script/Engine.StaticMeshComponent" "pullBar") (Math|Rotator|Lerp(Rotator) (Math|Rotator|MakeRotator (.roll _relativerotation_7) (.pitch _relativerotation_7) (.yaw _relativerotation_7)) (Math|Rotator|MakeRotator 13.333333 (.pitch _relativerotation_7) (.yaw _relativerotation_7)) _alpha_5 true) false false))
              (:Finished
                (goto _label_2))))
          (:3
            (bind _alpha_6 (Timeline|Timeline_5 PlayFromStart)
              (:Update
                (Transformation|SetRelativeRotation (Actor|GetComponentsbyTag (Variables|/Script/Engine.ChildActorComponent|GetChildActor (Variables|Default|GetChildActor)) "/Script/Engine.StaticMeshComponent" "pullBar") (Math|Rotator|Lerp(Rotator) (Math|Rotator|MakeRotator (.roll _relativerotation_8) (.pitch _relativerotation_8) (.yaw _relativerotation_8)) (Math|Rotator|MakeRotator 4e+01 (.pitch _relativerotation_8) (.yaw _relativerotation_8)) _alpha_6 true) false false))
              (:Finished
                (goto _label_2))))
          (:4
            (bind _alpha_7 (Timeline|Timeline PlayFromStart)
              (:Update
                (Transformation|SetRelativeRotation (Actor|GetComponentsbyTag (Variables|/Script/Engine.ChildActorComponent|GetChildActor (Variables|Default|GetChildActor)) "/Script/Engine.StaticMeshComponent" "pullBar") (Math|Rotator|Lerp(Rotator) "0.000000,0.000000,40.000000" "0.000000,0.000000,-40.000000" _alpha_7) false false))
              (:Finished
                (Variables|Default|SetReadyToInteract true)
                (Variables|Default|SetCurrent 1)
                (Class|BPIResponder|Respond(Message) (Variables|Default|GetConnectedActors) "NewEnumerator1" (Math|Conversions|ToFloat(Integer) (Variables|Default|GetCurrent)))))))
        (elif (== (Variables|Default|GetPositions) 5)
          (switch int (Variables|Default|GetCurrent)
            (:1
              ;[0.15 0.15 0.15 0.5] 5 Section
              (bind _alpha_8 (Timeline|Timeline_6 PlayFromStart)
                (:Update
                  (Transformation|SetRelativeRotation (Actor|GetComponentsbyTag (Variables|/Script/Engine.ChildActorComponent|GetChildActor (Variables|Default|GetChildActor)) "/Script/Engine.StaticMeshComponent" "pullBar") (Math|Rotator|Lerp(Rotator) (Math|Rotator|MakeRotator (.roll _relativerotation_2) (.pitch _relativerotation_2) (.yaw _relativerotation_2)) (Math|Rotator|MakeRotator -2e+01 (.pitch _relativerotation_2) (.yaw _relativerotation_2)) _alpha_8 true) false false))
                (:Finished
                  (Variables|Default|SetReadyToInteract true :!label _label_3)
                  (Variables|Default|SetCurrent (+ (Variables|Default|GetCurrent) 1))
                  (Class|BPIResponder|Respond(Message) (Variables|Default|GetConnectedActors) "NewEnumerator1" (Math|Conversions|ToFloat(Integer) (Variables|Default|GetCurrent))))))
            (:2
              (bind _alpha_9 (Timeline|Timeline_7 PlayFromStart)
                (:Update
                  (Transformation|SetRelativeRotation (Actor|GetComponentsbyTag (Variables|/Script/Engine.ChildActorComponent|GetChildActor (Variables|Default|GetChildActor)) "/Script/Engine.StaticMeshComponent" "pullBar") (Math|Rotator|Lerp(Rotator) (Math|Rotator|MakeRotator (.roll _relativerotation_5) (.pitch _relativerotation_5) (.yaw _relativerotation_5)) (Math|Rotator|MakeRotator 0.0 (.pitch _relativerotation_5) (.yaw _relativerotation_5)) _alpha_9 true) false false))
                (:Finished
                  (goto _label_3))))
            (:3
              (bind _alpha_10 (Timeline|Timeline_8 PlayFromStart)
                (:Update
                  (Transformation|SetRelativeRotation (Actor|GetComponentsbyTag (Variables|/Script/Engine.ChildActorComponent|GetChildActor (Variables|Default|GetChildActor)) "/Script/Engine.StaticMeshComponent" "pullBar") (Math|Rotator|Lerp(Rotator) (Math|Rotator|MakeRotator (.roll _relativerotation_9) (.pitch _relativerotation_9) (.yaw _relativerotation_9)) (Math|Rotator|MakeRotator 2e+01 (.pitch _relativerotation_9) (.yaw _relativerotation_9)) _alpha_10 true) false false))
                (:Finished
                  (goto _label_3))))
            (:4
              (bind _alpha_11 (Timeline|Timeline_9 PlayFromStart)
                (:Update
                  (Transformation|SetRelativeRotation (Actor|GetComponentsbyTag (Variables|/Script/Engine.ChildActorComponent|GetChildActor (Variables|Default|GetChildActor)) "/Script/Engine.StaticMeshComponent" "pullBar") (Math|Rotator|Lerp(Rotator) (Math|Rotator|MakeRotator (.roll _relativerotation) (.pitch _relativerotation) (.yaw _relativerotation)) (Math|Rotator|MakeRotator 4e+01 (.pitch _relativerotation) (.yaw _relativerotation)) _alpha_11 true) false false))
                (:Finished
                  (goto _label_3))))
            (:5
              (bind _alpha_12 (Timeline|Timeline_10 PlayFromStart)
                (:Update
                  (Transformation|SetRelativeRotation (Actor|GetComponentsbyTag (Variables|/Script/Engine.ChildActorComponent|GetChildActor (Variables|Default|GetChildActor)) "/Script/Engine.StaticMeshComponent" "pullBar") (Math|Rotator|Lerp(Rotator) "0.000000,0.000000,40.000000" "0.000000,0.000000,-40.000000" _alpha_12) false false))
                (:Finished
                  (Variables|Default|SetReadyToInteract true)
                  (Variables|Default|SetCurrent 1)
                  (Class|BPIResponder|Respond(Message) (Variables|Default|GetConnectedActors) "NewEnumerator1" (Math|Conversions|ToFloat(Integer) (Variables|Default|GetCurrent))))))))))))

(fn ConstructionScript
  (|CallParentFunction))