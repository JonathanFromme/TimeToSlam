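; BP_MI_LeverB is an interactable multi-position lever that plays a pull sound and animates its bar on each Interact.
; On BeginPlay it finds the child actor's mesh tagged pullBar and records its starting pitch.
; Each pull advances Current and runs a timeline one equal pitch step toward MaxRotation, then wraps to the start through a Reset timeline after the last position.
; ReadyToInteract blocks new pulls until the animation finishes.
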(event EventBeginPlay
  (|CallParentFunction)
  (for _array_element (Actor|GetComponentsbyTag (Variables|/Script/Engine.ChildActorComponent|GetChildActor (Variables|Default|GetChildActor)) "/Script/Engine.StaticMeshComponent" "pullBar")
    (bind _output_get (Variables|Default|SetpullBar _array_element))
    (bind _output_get_2 (Variables|Default|SetorigPos (Transformation|GetWorldRotation _output_get)))
    (Variables|Default|SetcurrentRotation (.pitch _output_get_2))))

(event Collision|EventActorBeginOverlap
  (params (OtherActor :type Actor%20Object%20Reference))
  (|CallParentFunction OtherActor) ; This node is disabled and will not be called.\nDrag off pins to build functionality.
)

(event EventTick
  (params (DeltaSeconds :type Float%20%28single-precision%29))
  (|CallParentFunction DeltaSeconds) ; This node is disabled and will not be called.\nDrag off pins to build functionality.
)

(event EventInteract
  (params (Amount :type Float%20%28double-precision%29))
  (if (Variables|Default|GetReadyToInteract)
    (Audio|SpawnSoundatLocation "/Game/TombFleeer/Sounds/Foley/MS_leverPull.MS_leverPull" (Transformation|GetActorLocation) "0, 0, 0" (Variables|Default|GetVolume%20Multiplier) 1.0 0.0 "/Game/TombFleeer/Sounds/Foley/Attenuation/SA_leverPull.SA_leverPull" 0)
    (Variables|Default|SetReadyToInteract false)
    (bind _output_get (Variables|Default|SetCurrent (+ (Variables|Default|GetCurrent) 1)))
    (if (<= _output_get (- (Variables|Default|GetPositions) 1))
      (bind _leveranimation (Timeline|SmallIncrement PlayFromStart)
        (:Update
          (Transformation|SetRelativeRotation (Variables|Default|GetpullBar) (Math|Rotator|MakeRotator 0.0 (.pitch (Math|Rotator|Lerp(Rotator) (Math|Rotator|MakeRotator 0.0 (Variables|Default|GetcurrentRotation) 0.0) (Math|Rotator|MakeRotator 0.0 (- (Variables|Default|GetcurrentRotation) (/ (- (.pitch (Variables|Default|GetorigPos)) (Variables|Default|GetMaxRotation)) (- (Variables|Default|GetPositions) 1))) 0.0) _leveranimation)) 0.0) false false))
        (:Finished
          (Variables|Default|SetcurrentRotation (- (Variables|Default|GetcurrentRotation) (/ (- (.pitch (Variables|Default|GetorigPos)) (Variables|Default|GetMaxRotation)) (- (Variables|Default|GetPositions) 1))))
          (Variables|Default|SetReadyToInteract true :!label _label)))
      (else
        (Variables|Default|SetCurrent 0)
        (bind _leveranimation_2 (Timeline|Reset PlayFromStart)
          (:Update
            (Transformation|SetRelativeRotation (Variables|Default|GetpullBar) (Math|Rotator|MakeRotator 0.0 (.pitch (Math|Rotator|Lerp(Rotator) (Math|Rotator|MakeRotator 0.0 (Variables|Default|GetcurrentRotation) 0.0) (Math|Rotator|MakeRotator 0.0 (.pitch (Variables|Default|GetorigPos)) 0.0) _leveranimation_2)) 0.0) false false))
          (:Finished
            (Variables|Default|SetcurrentRotation (.pitch (Variables|Default|GetorigPos)))
            (goto _label)))))))

(fn ConstructionScript
  (|CallParentFunction))