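; Interactable pillar in TombFleeer that counts toward or triggers the win condition when used.
; Interact reveals the "pullBar" mesh on its child actor, sets Activated, and sends RespondMessage to the first BP_VictoryText tagged "WinCon".
; CanInteract returns the ReadyToInteract flag, which this Blueprint's graphs never set.
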(event EventBeginPlay)

(event Collision|EventActorBeginOverlap
  (params (OtherActor :type Actor%20Object%20Reference)))

(event EventTick
  (params (DeltaSeconds :type Float%20%28single-precision%29)))

(event EventInteract
  (params (Amount :type Float%20%28double-precision%29))
  (Rendering|SetVisibility (Utilities|Array|Get(acopy) (Actor|GetComponentsbyTag (Variables|/Script/Engine.ChildActorComponent|GetChildActor (Variables|Default|GetChildActor)) "/Script/Engine.StaticMeshComponent" "pullBar")) true false)
  (Variables|Default|SetActivated true)
  (bind _outactors (Actor|GetAllActorsOfClasswithTag "/Game/TombFleeer/Responders/BP_VictoryText.BP_VictoryText_C" "WinCon"))
  (Class|BPIResponder|Respond(Message) (Utilities|Array|Get(acopy) _outactors) "NewEnumerator0" 0.0))

(fn ConstructionScript)

(fn CanInteract
  (return (Variables|Default|GetReadyToInteract)))