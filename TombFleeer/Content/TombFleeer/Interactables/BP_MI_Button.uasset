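; BP_MI_Button is an interactable button that triggers the actors connected to it.
; Interact plays a press sound and sends RespondMessage with its ControllerType to each connected actor whose CanRespondMessage passes.
; A Timeline then moves the child actor's "button"-tagged mesh between its BeginPlay position and a slightly lower one.
; ReadyToInteract blocks re-presses until the Timeline finishes, though CanInteract always returns true.
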(event EventBeginPlay
  (|CallParentFunction)
  (for _array_element (Actor|GetComponentsbyTag (Variables|/Script/Engine.ChildActorComponent|GetChildActor (Variables|Default|GetChildActor)) "/Script/Engine.StaticMeshComponent" "button")
    (Variables|Default|SetorigPosition (Transformation|GetWorldLocation _array_element))))

(event Collision|EventActorBeginOverlap
  (params (OtherActor :type Actor%20Object%20Reference))
  (|CallParentFunction OtherActor) ; This node is disabled and will not be called.\nDrag off pins to build functionality.
)

(event EventTick
  (params (DeltaSeconds :type Float%20%28single-precision%29))
  (|CallParentFunction DeltaSeconds) ; This node is disabled and will not be called.\nDrag off pins to build functionality.
)

(event EventInteract
  (params (Amount :type Float%20%28double-precision%29))
  (bind _origposition (Variables|Default|GetorigPosition))
  (if (Variables|Default|GetReadyToInteract)
    (Development|PrintString "Hello")
    (Variables|Default|SetReadyToInteract false)
    (Audio|SpawnSoundatLocation "/Game/TombFleeer/Sounds/Foley/MS_buttonPress.MS_buttonPress" (Transformation|GetActorLocation) "0, 0, 0" 1.0 1.0 0.25 "/Game/TombFleeer/Sounds/Foley/Attenuation/SA_buttonPress.SA_buttonPress" 0)
    (for _array_element (Variables|Default|GetConnectedActors)
      (bind _value (Class|BPIResponder|CanRespond(Message) _array_element))
      (if _value
        (Class|BPIResponder|Respond(Message) _array_element (Variables|Default|GetController%20Type) 0.0)))
    (bind _alpha (Timeline|Timeline PlayFromStart)
      (:Update
        (Transformation|SetWorldLocation (Actor|GetComponentsbyTag (Variables|/Script/Engine.ChildActorComponent|GetChildActor (Variables|Default|GetChildActor)) "/Script/Engine.StaticMeshComponent" "button") (Math|Vector|Lerp(Vector) _origposition (- _origposition "0.000000,0.000000,10.000000") _alpha) false false))
      (:Finished
        (Variables|Default|SetReadyToInteract true)))))

(fn ConstructionScript
  (|CallParentFunction))

(fn CanInteract
  (return true))