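; BP_MasterInteractable is a base interactable actor that provides highlight feedback on the object held in its ChildActor component.
; OnInteractHighlight applies a green overlay material to every static mesh component of that child actor, and OnInteractEnd clears it.
; CanInteract always returns false here, and the actor has no other active logic.
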(event EventBeginPlay)

(event Collision|EventActorBeginOverlap
  (params (OtherActor :type Actor%20Object%20Reference)))

(event EventTick
  (params (DeltaSeconds :type Float%20%28single-precision%29)))

(event EventOnInteractHighlight
  (for _array_element (Actor|GetComponentsByClass (Variables|/Script/Engine.ChildActorComponent|GetChildActor (Variables|Default|GetChildActor)) "/Script/Engine.StaticMeshComponent")
    (Rendering|Material|SetOverlayMaterial _array_element "/Game/TombFleeer/Materials/MI_GreenHighlight.MI_GreenHighlight" :!class /Script/Engine.MeshComponent)))

(event EventOnInteractEnd
  (for _array_element (Actor|GetComponentsByClass (Variables|/Script/Engine.ChildActorComponent|GetChildActor (Variables|Default|GetChildActor)) "/Script/Engine.StaticMeshComponent")
    (Rendering|Material|SetOverlayMaterial _array_element 0 :!class /Script/Engine.MeshComponent)))

(fn ConstructionScript)

(fn CanInteract
  (return false))