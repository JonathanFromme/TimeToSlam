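; Interactable dial that the player turns with horizontal mouse movement to drive connected actors.
; On BeginPlay it finds the "button"-tagged mesh inside its child actor and derives the starting yaw from it.
; Each Interact call adds scaled mouse delta to that yaw and sends the result to ConnectedActors through RespondMessage.
; When the yaw has changed, a DoOnce plays a short slice of the dial sound, then resets to throttle repeats.
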(event EventBeginPlay
  (|CallParentFunction)
  (for _array_element (Actor|GetComponentsbyTag (Variables|/Script/Engine.ChildActorComponent|GetChildActor (Variables|Default|GetChildActor)) "/Script/Engine.StaticMeshComponent" "button")
    (bind _output_get (Variables|Default|SetDial _array_element))
    (bind _output_get_2 (Variables|Default|SetorigRot (Transformation|GetWorldRotation _output_get)))
    (Variables|Default|SetcurrentRot (- (.yaw _output_get_2) 9e+01))))

(event Collision|EventActorBeginOverlap
  (params (OtherActor :type Actor%20Object%20Reference))
  (|CallParentFunction OtherActor) ; This node is disabled and will not be called.\nDrag off pins to build functionality.
)

(event EventTick
  (params (DeltaSeconds :type Float%20%28single-precision%29))
  (|CallParentFunction DeltaSeconds) ; This node is disabled and will not be called.\nDrag off pins to build functionality.
)

(event EventInteract
  (params (Amount :type Float%20%28double-precision%29))
  (Utilities|FlowControl|Sequence
    (:then_0
      (if (!= (Variables|Default|GetpreviousFrame) (Variables|Default|GetcurrentRot))
        (Variables|Default|SetpreviousFrame (Variables|Default|GetcurrentRot))
        (Utilities|FlowControl|DoOnce false :!label _label
          (:Completed
            (bind _returnvalue (Audio|SpawnSoundAttached "/Game/TombFleeer/Sounds/Foley/MS_Dial.MS_Dial" (Variables|Default|GetChildActor) "None" "0, 0, 0" "0, 0, 0" "KeepRelativeOffset" false 1.0 1.0 0.5 "/Game/TombFleeer/Sounds/Foley/Attenuation/SA_buttonPress.SA_buttonPress" 0))
            (Utilities|FlowControl|Delay 0.2)
            (Audio|Components|Audio|Stop _returnvalue)
            (goto _label Reset)))))
    (:then_1
      (Transformation|SetRelativeRotation (Variables|Default|GetDial) (Math|Rotator|MakeRotator 0.0 0.0 (+ (Variables|Default|GetcurrentRot) (.yaw (Math|Rotator|MakeRotator 0.0 0.0 (* (.DeltaX (Class|PlayerController|GetInputMouseDelta (Game|GetPlayerController 0))) 1e+01))))) false false)
      (Class|BPIResponder|Respond(Message) (Variables|Default|GetConnectedActors) "NewEnumerator2" (.yaw (Variables|/Script/Engine.SceneComponent|GetRelativeRotation (Variables|Default|GetDial))))
      (Variables|Default|SetcurrentRot (.yaw (Variables|/Script/Engine.SceneComponent|GetRelativeRotation (Variables|Default|GetDial)))))))

(fn ConstructionScript
  (|CallParentFunction))