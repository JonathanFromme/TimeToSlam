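; BP_MI_Scales is an interactable that relays player interaction to a child actor, by its name a set of scales.
; Highlight events apply or clear a green overlay material on that actor's SM_jug_02 mesh, found by object name.
; Interact forwards the amount through InteractMessage, plays an attenuated stone-drop sound at the InputJar-tagged mesh, and blocks readiness for a half-second cooldown.
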(event EventBeginPlay
  (|CallParentFunction) ; This node is disabled and will not be called.\nDrag off pins to build functionality.
)

(event Collision|EventActorBeginOverlap
  (params (OtherActor :type Actor%20Object%20Reference))
  (|CallParentFunction OtherActor) ; This node is disabled and will not be called.\nDrag off pins to build functionality.
)

(event EventTick
  (params (DeltaSeconds :type Float%20%28single-precision%29))
  (|CallParentFunction DeltaSeconds) ; This node is disabled and will not be called.\nDrag off pins to build functionality.
)

(event EventOnInteractHighlight
  (for _array_element (Actor|GetComponentsByClass (Variables|/Script/Engine.ChildActorComponent|GetChildActor (Variables|Default|GetChildActor)) "/Script/Engine.StaticMeshComponent")
    (if (Utilities|Enum|Equal(Enum) (Utilities|GetObjectName _array_element) "SM_jug_02")
      (Rendering|Material|SetOverlayMaterial _array_element "/Game/TombFleeer/Materials/MI_GreenHighlight.MI_GreenHighlight" :!class /Script/Engine.MeshComponent))))

(event EventInteract
  (params (Amount :type Float%20%28double-precision%29))
  (Variables|Default|SetReadyToInteract false)
  (Class|BPIInteract|Interact(Message) (Variables|/Script/Engine.ChildActorComponent|GetChildActor (Variables|Default|GetChildActor)) Amount)
  (Audio|SpawnSoundatLocation "/Game/TombFleeer/Sounds/Foley/StoneDrop/MS_StoneDrop.MS_StoneDrop" (Transformation|GetWorldLocation (Utilities|Array|Get(acopy) (Actor|GetComponentsbyTag (Variables|/Script/Engine.ChildActorComponent|GetChildActor (Variables|Default|GetChildActor)) "/Script/Engine.StaticMeshComponent" "InputJar"))) "0, 0, 0" 1.0 1.0 0.0 "/Game/TombFleeer/Sounds/Foley/StoneDrop/SA_stoneDrop.SA_stoneDrop" 0)
  (Utilities|FlowControl|Delay 0.5)
  (Variables|Default|SetReadyToInteract true))

(event EventOnInteractEnd
  (for _array_element (Actor|GetComponentsByClass (Variables|/Script/Engine.ChildActorComponent|GetChildActor (Variables|Default|GetChildActor)) "/Script/Engine.StaticMeshComponent")
    (if (Utilities|Enum|Equal(Enum) (Utilities|GetObjectName _array_element) "SM_jug_02")
      (Rendering|Material|SetOverlayMaterial _array_element 0 :!class /Script/Engine.MeshComponent))))

(fn ConstructionScript
  (|CallParentFunction))