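; BP_Button is an interactable button that highlights and animates when used, with no other effect triggered in its graphs.
; Highlight and end-interaction events set and clear a green overlay material on its Cylinder.
; Interact plays a Timeline that lerps the Cylinder's relative height to animate the press.
; A ReadyToInteract flag, exposed through CanInteract, blocks re-triggering until the Timeline finishes.
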(event EventBeginPlay)

(event Collision|EventActorBeginOverlap
  (params (OtherActor :type Actor%20Object%20Reference)))

(event EventTick
  (params (DeltaSeconds :type Float%20%28single-precision%29)))

(event EventOnInteractEnd
  (Rendering|Material|SetOverlayMaterial (Variables|Default|GetCylinder) 0 :!class /Script/Engine.MeshComponent))

(event EventOnInteractHighlight
  (Rendering|Material|SetOverlayMaterial (Variables|Default|GetCylinder) "/Game/TombFleeer/Materials/MI_GreenHighlight.MI_GreenHighlight" :!class /Script/Engine.MeshComponent))

(event EventInteract
  (if (Variables|Default|GetReadyToInteract)
    (Variables|Default|SetReadyToInteract false)
    (bind _alpha (Timeline|Timeline PlayFromStart)
      (:Update
        (Transformation|SetRelativeLocation (Variables|Default|GetCylinder) (Math|Vector|Lerp(Vector) "0.000000,0.000000,10.000000" "0.000000,0.000000,-10.000000" _alpha) false false))
      (:Finished
        (Variables|Default|SetReadyToInteract true)))))

(fn ConstructionScript)

(fn CanInteract
  (return (Variables|Default|GetReadyToInteract)))